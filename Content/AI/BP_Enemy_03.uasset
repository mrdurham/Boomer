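; Enemy character that spots the player with PawnSensing, moves toward and faces them, and deals damage on actor overlap.
; Tick detects hits by comparing Health to a cached LocalHP, triggering a nudge, sound and material flicker, while turning the HP bar toward the player.
; At zero health it enables box physics, removes the bar, blinks and destroys itself.
; Burst projectile fire is disconnected, and slope-speed and grapple helper functions are never called here.
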(event `self.ReceiveActorBeginOverlap`
  (params (OtherActor :type "Actor Object Reference"))
  (`KismetSystemLibrary.PrintString` "CONE D A M A G I N G")
  (message `/Game/FirstPerson/Blueprints/BPI_Damagable.Take Damage` OtherActor 10.0))

(event `self.ReceiveBeginPlay`
  (bind _asui_hpbar (cast `/Game/UI_HPBar` (`WidgetComponent.GetWidget` (`self.hp`))))
  (set `/Game/UI_HPBar.Enemy3` self _asui_hpbar))

(event `self.ReceiveTick`
  (params (DeltaSeconds :type "Float (single-precision)"))
  (if (`self.IsDamaged`)
    (`self.NudgeWhenHit`)
    (`GameplayStatics.PlaySound2D` "/Game/Shotgun_fire_01.Shotgun_fire_01" 0.5 2.0 0.1 null null)
    (`self.FlashOn`)
    (`KismetSystemLibrary.Delay` (`KismetMathLibrary.RandomFloatInRange` 0.01 0.033))
    (`self.BlinkOn`)
    (`KismetSystemLibrary.Delay` (`KismetMathLibrary.RandomFloatInRange` 0.075 0.12))
    (`self.FlashOn`)
    (`KismetSystemLibrary.Delay` (`KismetMathLibrary.RandomFloatInRange` 0.07 0.1))
    (`self.BlinkOn`))
  (set `self.Local_HP` (`self.Health`))
  (`SceneComponent.K2_SetWorldRotation` (`self.hp`) (`KismetMathLibrary.FindLookAtRotation` (`SceneComponent.GetSocketLocation` (`self.hp`) "None") (`SceneComponent.K2_GetComponentLocation` (`Character.CapsuleComponent` (`GameplayStatics.GetPlayerCharacter` 0)))) false false)
  (if (<= (`self.Health`) 0.0)
    (`/Engine/EditorBlueprintResources/StandardMacros.DoOnce` false
      (:`Completed`
        (`PrimitiveComponent.SetSimulatePhysics` (`self.Box`) true)
        (`ActorComponent.K2_DestroyComponent` (`self.hp`))
        (`self.BlinkOff`)
        (`KismetSystemLibrary.Delay` 0.2)
        (`self.BlinkOn`)
        (`KismetSystemLibrary.Delay` 0.1)
        (`self.BlinkOff`)
        (`KismetSystemLibrary.Delay` 0.05)
        (`self.BlinkOn`)
        (`KismetSystemLibrary.Delay` 0.15)
        (`self.BlinkOff`)
        (`KismetSystemLibrary.Delay` 3.0)
        (`self.BlinkOff`)
        (`KismetSystemLibrary.Delay` 2.0)
        (`self.K2_DestroyActor`)))
    (elif (`self.HasPlayer`)
      (bind _asbp_first_person_character (cast `/Game/FirstPerson/Blueprints/BP_FirstPersonCharacter` (`self.SeenPawn`)))
      (`|ExecutionSequence`
        (:`then_0`
          (`self.K2_SetActorRotation` (`KismetMathLibrary.FindLookAtRotation` (`self.K2_GetActorLocation`) (`self.K2_GetActorLocation` _asbp_first_person_character))))))))

(event `self.PawnSensing.OnSeePawn`
  (params (Pawn :type "Pawn Object Reference"))
  (bind _output_get (set `self.SeenPawn` Pawn))
  (bind _asbp_first_person_character (cast `/Game/FirstPerson/Blueprints/BP_FirstPersonCharacter` _output_get))
  (set `self.HasPlayer` true)
  (`|AIMoveTo` self (`SceneComponent.K2_GetComponentLocation` (`Character.CapsuleComponent` _asbp_first_person_character)) _output_get))

(fn `BlinkOff`
  (`PrimitiveComponent.SetMaterial` (`self.Cone`) 0 "/Engine/BasicShapes/EnemyMaterial_4_dark.EnemyMaterial_4_dark"))

(fn `BlinkOn`
  (`PrimitiveComponent.SetMaterial` (`self.Cone`) 0 "/Engine/BasicShapes/EnemyMaterial_4.EnemyMaterial_4"))

(fn `BurstFire`
  (locals (CurrentBurst :type Integer)))

(fn `FlashOn`
  (`PrimitiveComponent.SetMaterial` (`self.Cone`) 0 "/Engine/BasicShapes/EnemyMaterial_3.EnemyMaterial_3"))

(fn `Get_Angle_Speed`
  (returns (`Desired Speed` :type "Float (double-precision)"))
  (locals (Speed :type "Float (single-precision)" :default 0.0))
  ;[1 1 1] get angle speed - get our floor angle - get value from our curve
  (set `local.Speed` (`CurveFloat.GetFloatValue` (`self.float Curve`) (.pitch (`KismetMathLibrary.FindLookAtRotation` (`self.Previous_Location`) (`self.K2_GetActorLocation`)))))
  (set `self.Previous_Location` (`self.K2_GetActorLocation`))
  (return (`local.Speed`)))

(fn `Grapple positioning`
  (returns (ReturnValue :type "Vector Structure"))
  (return (* (`KismetMathLibrary.Normal` (+ (`KismetMathLibrary.GetDirectionUnitVector` (`self.K2_GetActorLocation`) (`self.GrapplePointLocation`)) (* (* (`self.GetActorRightVector`) (`self.GetInputAxisValue`)) 0.5))) 3200000.0)))

(fn `IsDamaged`
  (returns (ReturnValue :type Boolean))
  (return (> (`self.Local_HP`) (`self.Health`))))

(fn `NudgeWhenHit`
  (`SceneComponent.K2_AddWorldOffset` (`self.CapsuleComponent`) (`KismetMathLibrary.MakeVector` (`KismetMathLibrary.RandomFloatInRange` -50.0 50.0) (`KismetMathLibrary.RandomFloatInRange` -20.0 20.0)) true false))

(fn `Should_Update_speed`
  (returns (`Should Update` :type Boolean))
  (bind _charactermovement (`self.CharacterMovement`))
  ;[1 1 1] should update - not falling - have velocity
  (return (and (not (`NavMovementComponent.IsFalling` _charactermovement)) (> (`KismetMathLibrary.VSizeSquared` (`MovementComponent.Velocity` _charactermovement)) 0.0))))

(fn `Trace and hit`
  (returns (OutHit :type "HitResult Structure") (HIt :type Boolean))
  (bind _returnvalue (`GameplayStatics.GetPlayerCameraManager` 0))
  (bind _returnvalue_2 (`PlayerCameraManager.GetCameraLocation` _returnvalue))
  (bind (_outhit _returnvalue_3) (`KismetSystemLibrary.LineTraceSingleForObjects` _returnvalue_2 (+ _returnvalue_2 (* (`self.GetActorForwardVector` _returnvalue) 10000.0)) (`|MakeArray` "ObjectTypeQuery8" :!type "EObjectTypeQuery Enum")))
  (return _outhit _returnvalue_3))

(fn `Update_Char_speed`
  (bind _should_update (`self.Should_Update_speed`))
  (if _should_update
    (bind _desired_speed (`self.Get_Angle_Speed`))
    (`self.Update_Movement_Speed` _desired_speed)))

(fn `Update_Movement_Speed`
  (params (`Desired Speed` :type "Float (double-precision)"))
  ;[1 1 1] update to desired speed
  (set `CharacterMovementComponent.MaxWalkSpeed` (`KismetMathLibrary.FInterpTo` (`CharacterMovementComponent.MaxWalkSpeed` (`self.CharacterMovement`)) `Desired Speed` (`self.Delta Time`) (`self.Desired speed rate`)) (`self.CharacterMovement`)))

(fn `UserConstructionScript`)